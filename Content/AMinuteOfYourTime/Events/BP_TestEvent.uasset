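; BP_TestEvent is an event Blueprint, apparently for testing, that presents an event as pages in the journal.
; Execute checks the caller, runs the parent logic, then has the journal subsystem push header and event pages and start the event path.
; The header receives the event description, and an invalid caller raises a script error.
; Reaching the path end notifies the player HUD that the event is complete.
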(event `StoryEventInterface.Execute`
  (params (EventDescription :type "EventDescriptionRow Structure") (Caller :type "Object Object Reference"))
  (`/Engine/EditorBlueprintResources/StandardMacros.IsValid` Caller
    (:`Is Valid`
      (`parent.Execute` EventDescription Caller)
      (bind _returnvalue (`JournalSubsystem.PushPagesAndStartPath` (`JournalSubsystem.GetJournalSubsystem` Caller) (`|MakeArray` "/Game/AMinuteOfYourTime/UserInterface/Event/WBP_EventHeader.WBP_EventHeader_C" "/Game/AMinuteOfYourTime/UserInterface/Event/WBP_EventPage.WBP_EventPage_C" :!type "UserWidget Class Reference") (`self.EventPath`)))
      (message `/Game/AMinuteOfYourTime/Events/BPI_EventHandler.Initialize` (`|GetArrayItem` _returnvalue) EventDescription))
    (:`Is Not Valid`
      (`KismetSystemLibrary.RaiseScriptError` "CALLING EVENT WITH INVALID CALLER"))))

(event `StoryEventInterface.OnPathEndReached`
  (params (PathName :type String) (CurrentHandler :type "Object Object Reference"))
  (`/Game/AMinuteOfYourTime/UserInterface/WBP_PlayerHUD.OnEventComplete` (`self.PlayerHUD`)))
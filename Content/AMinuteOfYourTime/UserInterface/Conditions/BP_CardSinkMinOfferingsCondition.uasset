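; Card sink condition for the Crucible UI that checks whether enough offerings are placed for a card's ability.
; Evaluate passes when the sink's card count reaches the minimum of the ability's min/max offerings range, read through the card ability system.
; It expects a WBP_Crucible as user data and otherwise raises a script error and fails.
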(fn `Evaluate`
  (params (CardSink :type "/Game/AMinuteOfYourTime/UserInterface/Cards/WBP_CardSink Object Reference") (Card :type "/Game/AMinuteOfYourTime/UserInterface/Cards/WBP_Card Object Reference") (UserData :type "Object Object Reference"))
  (returns (Allow :type Boolean))
  (bind _returnvalue_x (`KismetMathLibrary.BreakVector2D` (`CardAbilitySystem.GetAbilityMinMaxOfferings` (`CardAbilitySystem.GetCardAbilitySystem` Card) (`CardDataBase.Card` (`/Game/AMinuteOfYourTime/UserInterface/Cards/VM_Card.CardDataRef` (`/Game/AMinuteOfYourTime/UserInterface/Cards/WBP_Card.VM_Card` Card))))))
  (cast `/Game/AMinuteOfYourTime/UserInterface/WBP_Crucible` UserData
    (:`then`
      (return (>= (`KismetArrayLibrary.Array_Length` (`/Game/AMinuteOfYourTime/UserInterface/Cards/WBP_CardSink.GetAllCards` CardSink false)) _returnvalue_x)))
    (:`CastFailed`
      (`KismetSystemLibrary.RaiseScriptError` "EXPECTED USER DATA TO BE CRUCIBLE, BUT IT WASN'T")
      (return false))))